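; Game state Blueprint that tracks XP and level, driving the XP bar and level-up screen.
; Server_AddXP accumulates XP, pauses the game on reaching the threshold, then loops through level-ups, carrying leftover XP over an exponentially growing requirement.
; Multicast events update player controller 0's HUD bar and show one level-up widget per XP gain, even when several levels are earned.
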(event Custom|Multicast_UpdateUI_XP
  (params (CurrentXP :type Float%20%28double-precision%29) (RequiredXP :type Float%20%28double-precision%29))
  ;[1 1 1] Multicast UI Update - Must run on Server
  (bind _asbp_mgb_player_controller (Utilities|Casting|CastToBP_MgbPlayerController (Game|GetPlayerController 0)))
  (Default|UpdateXPBar (Variables|/Game/Blueprints/Player/BP_MgbPlayerController.BP_MgbPlayerController_C|GetGameHUD _asbp_mgb_player_controller) (/ CurrentXP RequiredXP)))

(event Custom|Server_AddXP
  (params (In%20XP :type Float%20%28double-precision%29))
  ;[1 1 1] Run on Server XPGain
  (bind _output_get (Variables|Default|SetCurrentXP (+ In%20XP (Variables|Default|GetCurrentXP))))
  (if (>= _output_get (Variables|Default|GetRequiredXP))
    (CallFunction|MulticastUpdateUIXP (Variables|Default|GetCurrentXP) (Variables|Default|GetRequiredXP))
    (Game|SetGamePaused true)
    (CallFunction|MulticastLevelUp)
    ;;[1 1 1] Remaining XP 처리
    (while (>= (Variables|Default|GetCurrentXP) (Variables|Default|GetRequiredXP))
      (Math|Integer|IncrementInt (Variables|Default|GetCurrentLevel)
        (:%20%20
          (Variables|Default|SetCurrentXP (- (Variables|Default|GetCurrentXP) (Variables|Default|GetRequiredXP)))
          (Variables|Default|SetRequiredXP (* 1e+02 (Math|Float|Power 1.2 (Math|Conversions|ToFloat(Integer) (- (Variables|Default|GetCurrentLevel) 1))))))))
    (CallFunction|MulticastUpdateUIXP (Variables|Default|GetCurrentXP) (Variables|Default|GetRequiredXP))
    (else
      (CallFunction|MulticastUpdateUIXP (Variables|Default|GetCurrentXP) (Variables|Default|GetRequiredXP)))))

(event Custom|Multicast_LevelUp
  (bind _returnvalue (UserInterface|CreateWidget "/Game/Blueprints/UI/WB_TEST_Levelup.WB_TEST_Levelup_C" (Game|GetPlayerController 0)))
  (UserInterface|Viewport|AddtoViewport _returnvalue 0))

(fn ConstructionScript)