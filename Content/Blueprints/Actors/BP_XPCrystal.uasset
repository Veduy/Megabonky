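; XP crystal pickup that turns to face the local player camera every tick and flies to whoever picks it up.
; On the server, BeginPlay binds ActionEvent to OnAction, storing the target so Tick lerps toward it with growing alpha.
; Server-side sphere overlap with a player character pawn adds XP through the game state and destroys the crystal.
; An older timeline-driven hop-then-pull handler remains but is never bound.
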(event OnComponentBeginOverlap(Sphere)
  (params (OverlappedComponent :type Primitive%20Component%20Object%20Reference) (OtherActor :type Actor%20Object%20Reference) (OtherComp :type Primitive%20Component%20Object%20Reference) (OtherBodyIndex :type Integer) (bFromSweep :type Boolean) (SweepResult :type Hit%20Result%20Structure%20%28by%20ref%29))
  ;[1 1 1] Only Server Update XP
  (if (Ability|HasAuthority)
    (switch Utilities|FlowControl|Switch|SwitchonECollisionChannel (Collision|GetCollisionObjectType OtherComp)
      (:ECC_Pawn
        (Utilities|Casting|CastToBP_MgbPlayerCharacter OtherActor)
        (bind _asbp_mgb_game_state_base (Utilities|Casting|CastToBP_MgbGameStateBase (Game|GetGameState)))
        (Class|MgbGameStateBase|ServerAddXP _asbp_mgb_game_state_base 2e+01)
        (Actor|DestroyActor)))))

(event Custom|ActionEvent
  (params (TargetActor :type Actor%20Object%20Reference))
  ;[0.15 0.15 0.15 0.5] Comment
  (Variables|Default|SetPickupActor TargetActor)
  (Variables|Default|SetbPicked true))

(event Custom|OnAction_Event
  (params (TargetActor :type Actor%20Object%20Reference))
  ;[0.15 0.15 0.15 0.5] Comment
  (Variables|Default|SetPickupActor TargetActor)
  (Utilities|FlowControl|DoOnce false :!label _label
    (:Completed
      (bind _pickupactor (Variables|Default|GetPickupActor)
        (:then
          (bind _height (Timeline|Pickup Play)
            (:Update
              (Transformation|AddActorWorldOffset (Math|Vector|MakeVector (.x (* (Class|KismetMathLibrary|VectorNormal2D (- (Transformation|GetActorLocation _pickupactor) (Transformation|GetActorLocation)) 0.0001) -1.0)) (.y (* (Class|KismetMathLibrary|VectorNormal2D (- (Transformation|GetActorLocation _pickupactor) (Transformation|GetActorLocation)) 0.0001) -1.0)) (+ (* _height 5.0) (.z (* (Class|KismetMathLibrary|VectorNormal2D (- (Transformation|GetActorLocation _pickupactor) (Transformation|GetActorLocation)) 0.0001) -1.0))))))
            (:Finished
              (Utilities|FlowControl|DoOnce false
                (:Completed
                  (bind _newtrack_0 (Timeline|Timeline Play)
                    (:Update
                      (bind _pickupactor_2 (Variables|Default|GetPickupActor)
                        (:then
                          (Transformation|SetActorLocation (Math|Vector|MakeVector (.x (Math|Vector|Lerp(Vector) (Transformation|GetActorLocation) (Transformation|GetActorLocation _pickupactor_2) _newtrack_0)) (.y (Math|Vector|Lerp(Vector) (Transformation|GetActorLocation) (Transformation|GetActorLocation _pickupactor_2) _newtrack_0)) (.z (Math|Vector|Lerp(Vector) (Transformation|GetActorLocation) (Transformation|GetActorLocation _pickupactor_2) _newtrack_0))) false false))
                        (:else)))))))))
        (:else
          (goto _label Reset))))))

(event EventBeginPlay
  ;[0.15 0.15 0.15 0.5] Comment
  (if (Ability|HasAuthority)
    (EventDispatchers|AssignOnAction (delegate Custom|ActionEvent))))

(event EventTick
  (params (DeltaSeconds :type Float%20%28single-precision%29))
  (bind _returnvalue (Game|GetPlayerController 0))
  (Utilities|FlowControl|Sequence
    (:then_0
      ;[0.15 0.15 0.15 0.5] Tick 항상 카메라를 바라보도록
      (Utilities|IsValid _returnvalue
        (:Is%20Valid
          (Transformation|SetActorRotation (Math|Rotator|FindLookatRotation (Transformation|GetActorLocation) (Camera|GetCameraLocation (Variables|/Script/Engine.PlayerController|GetPlayerCameraManager _returnvalue)))))))
    (:then_1
      ;[0.15 0.15 0.15 0.5] Comment
      (if (Variables|Default|GetbPicked)
        (bind _pickupactor (Variables|Default|GetPickupActor)
          (:then
            (Variables|Default|SetAlpha (+ (Variables|Default|GetAlpha) (* (Utilities|Time|GetWorldDeltaSeconds) 0.1)))
            (Transformation|SetActorLocation (Math|Vector|MakeVector (.x (Math|Vector|Lerp(Vector) (Transformation|GetActorLocation) (Transformation|GetActorLocation _pickupactor) (Variables|Default|GetAlpha))) (.y (Math|Vector|Lerp(Vector) (Transformation|GetActorLocation) (Transformation|GetActorLocation _pickupactor) (Variables|Default|GetAlpha))) (.z (Math|Vector|Lerp(Vector) (Transformation|GetActorLocation) (Transformation|GetActorLocation _pickupactor) (Variables|Default|GetAlpha)))) false false))
          (:else))))))

(fn ConstructionScript)