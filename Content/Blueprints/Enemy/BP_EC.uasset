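; BP_EC is an enemy Blueprint that adds hit feedback to the damage handling of its parent class.
; On each damage effect it spawns an attached yellow blood-impact Niagara system on its root component.
; It then reads Health from the EnemyAttributeSet on its Gameplay Ability System component and plays a hit sound at its location when the base value is zero or below.
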(event EventHandleDamageEffect
  (Niagara|SpawnSystemAttached "/Game/Assets/Effects/Combat/NS_BloodImpact_yellow.NS_BloodImpact_yellow" (Variables|Transformation|GetRootComponent) "None" "0, 0, 0" "0, 0, 0" "KeepRelativeOffset" true)
  (bind _returnvalue (GameplayAttributes|GetAttributeSet (Variables|Default|GetAbilitySystemComponent) "/Script/Megabonky.EnemyAttributeSet"))
  (if (<= (.BaseValue (Utilities|Struct|BreakGameplayAttributeData (Variables|/Script/Megabonky.EnemyAttributeSet|GetHealth _returnvalue))) 0.0)
    (Audio|PlaySoundatLocation "/Game/Assets/Megabonk/Sound/Hit2_0.Hit2_0" (Transformation|GetActorLocation) "0, 0, 0" 0.7 1.0 0.0 0 0 0 0)))

(event EventBeginPlay
  (|CallParentFunction))

(fn ConstructionScript)