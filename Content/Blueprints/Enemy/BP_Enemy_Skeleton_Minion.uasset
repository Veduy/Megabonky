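; BP_Enemy_Skeleton_Minion is the Blueprint for a skeleton minion enemy.
; On BeginPlay, only the authority starts a looping timer that calls CheckWall by name after an initial delay; that function is not defined in this graph.
; The capsule hit event is empty, and a disconnected, never-run branch holds logic to knock a player character away with a movement impulse.
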(event OnComponentHit(CapsuleComponent)
  (params (HitComponent :type Primitive%20Component%20Object%20Reference) (OtherActor :type Actor%20Object%20Reference) (OtherComp :type Primitive%20Component%20Object%20Reference) (NormalImpulse :type Vector :default "0, 0, 0") (Hit :type Hit%20Result%20Structure%20%28by%20ref%29)))

(event EventBeginPlay
  (Networking|SwitchHasAuthority
    (:Authority
      (Utilities|Time|SetTimerbyFunctionName 0 "CheckWall" 0.2 true false 2.0))))

(fn ConstructionScript)