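; Enemy Blueprint that animates its static mesh flipbook-style by swapping through an array of meshes.
; BeginPlay calls the parent and caches the last mesh index, and Tick runs PlayAnimation once SpawnFinished is set.
; PlayAnimation accumulates delta time to advance the frame at a fixed interval, wrapping by modulo on that last index, so the final mesh in the array is never shown.
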(event EventBeginPlay
  (|CallParentFunction)
  ;[0.15 0.15 0.15 0.5] Comment
  (Variables|StopAnim|SetMaxMeshFrame (- (Utilities|Array|Length (Variables|StopAnim|GetMeshes)) 1)))

(event EventTick
  (params (DeltaSeconds :type Float%20%28single-precision%29))
  (|CallParentFunction DeltaSeconds)
  (if (Variables|Default|GetbSpawnFinished)
    (CallFunction|PlayAnimation)))

(fn ConstructionScript)

(fn PlayAnimation
  ;[0.15 0.15 0.15 0.5] Comment
  (bind _output_get (Variables|StopAnim|SetFrameTime (+ (Utilities|Time|GetWorldDeltaSeconds) (Variables|StopAnim|GetFrameTime))))
  (if (> _output_get 0.2)
    (bind _result (Math|Integer|IncrementInt (Variables|StopAnim|GetCurMeshFrame))
      (:%20%20
        (Components|StaticMesh|SetStaticMesh (Variables|Default|GetStaticMesh) (Utilities|Array|Get(acopy) (Variables|StopAnim|GetMeshes) (Math|Integer|%(Integer) _result (Variables|StopAnim|GetMaxMeshFrame))))
        (Variables|StopAnim|SetFrameTime 0.0)))))