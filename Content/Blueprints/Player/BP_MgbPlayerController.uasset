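; BP_MgbPlayerController is a player controller that sets up mouse input and the in-game UI for the local player.
; On BeginPlay, local controllers switch to Game and UI input mode with the cursor shown and kept visible during capture.
; They then create a WB_InGame widget, store it as InGameWidget and add it to the viewport.
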(event EventBeginPlay
  (Utilities|FlowControl|Sequence
    (:then_0
      ;[1 1 1] Input Mode
      (if (Pawn|IsLocalPlayerController)
        (Input|SetInputModeGameandUI self 0 "DoNotLock" false false)
        (Variables|Default|SetbShowMouseCursor true)))
    (:then_1
      ;[0.15 0.15 0.15 0.5] Comment
      (if (Pawn|IsLocalPlayerController)
        (bind _returnvalue (UserInterface|CreateWidget "/Game/Blueprints/UI/InGame/WB_InGame.WB_InGame_C" self))
        (bind _output_get (Variables|Default|SetInGameWidget _returnvalue))
        (UserInterface|Viewport|AddtoViewport _output_get 0)))))

(fn ConstructionScript)