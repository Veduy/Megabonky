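; Player character Blueprint that adds death and landing feedback.
; DeathFadeOut plays a sound, pauses mesh animation and drives a blackout post-process material's Radius by timeline, then shows the game-over widget.
; OnLanded plays a camera shake for the locally controlled player above a speed threshold.
; A debug key draws a sphere trace at the primary target; unreachable example graphs sketch tome upgrades applied through a SetByCaller GameplayEffect.
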(event EventOnLanded
  (params (Hit :type Hit%20Result%20Structure%20%28by%20ref%29))
  ;[0.15 0.15 0.15 0.5 60] Landed Camera Shake
  (if (and (Pawn|IsLocallyControlled) (> (Math|Vector|VectorLength (Pawn|Components|CharacterMovement|GetLastUpdateVelocity (Variables|Character|GetCharacterMovement))) 4e+02))
    (Camera|PlayWorldCameraShake "/Game/Blueprints/CameraShake/CS_Landed.CS_Landed_C" (Transformation|GetActorLocation) 0.0 (Variables|/Script/Engine.SpringArmComponent|GetTargetArmLength (Variables|Default|GetSpringArm)) 0.0)))

(event EventDeathFadeOut
  ;[0.15 0.15 0.15 0.5 50] 캐릭터 사망시 연출(화면 어두워지는)
  (bind _returnvalue (Rendering|Material|CreateDynamicMaterialInstance "/Game/Blueprints/Materials/PPM_Blackout_Inst.PPM_Blackout_Inst" "" "None" :!class /Script/Engine.KismetMaterialLibrary))
  (bind _output_get (Variables|Default|SetPPM_ _returnvalue))
  (Rendering|AddorUpdateBlendable (Variables|Default|GetMainCamera) _output_get 1.0 :!class /Script/Engine.CameraComponent)
  (Utilities|FlowControl|Sequence
    (:then_0
      (bind _newtrack_0 (Timeline|Timeline PlayFromStart)
        (:Update
          (Rendering|Material|SetScalarParameterValue _returnvalue "Radius" _newtrack_0 :!class /Script/Engine.MaterialInstanceDynamic))
        (:Finished
          (bind _returnvalue_2 (UserInterface|CreateWidget "/Game/Blueprints/UI/InGame/WB_GameOver.WB_GameOver_C" (Game|GetPlayerController 0)))
          (UserInterface|Viewport|AddtoViewport _returnvalue_2 0))))
    (:then_1
      (Audio|PlaySound2D "/Game/Assets/Megabonk/AudioClip/DeathImpact.DeathImpact" 1.0 1.0 0.0 0 0)
      (Variables|/Script/Engine.SkeletalMeshComponent|SetbPauseAnims (Variables|Character|GetMesh) true))))

(event Input|KeyboardEvents|DebugKey2
  (params (Key :type Key%20Structure :default "None") (ActionValue :type Input%20Action%20Value%20Structure))
  ;[0.15 0.15 0.15 0.5] Primary Target 확인용
  (:Pressed
    (bind (_outprimarytarget _returnvalue) (Class|MgbPlayerCharacter|FindPrimaryTargetbyCondition))
    (if _returnvalue
      (Collision|SphereTraceByChannel (Transformation|GetActorLocation _outprimarytarget) (Transformation|GetActorLocation _outprimarytarget) 3e+01 "TraceTypeQuery1" false (Utilities|Array|MakeArray 0) "ForDuration" true "(R=1.000000,G=0.000000,B=0.000000,A=1.000000)" "(R=0.000000,G=1.000000,B=0.000000,A=1.000000)" 3.0))))

(fn ConstructionScript)