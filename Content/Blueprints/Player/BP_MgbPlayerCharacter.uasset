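; Player character Blueprint that sets up its Gameplay Ability System attributes and holds prototype upgrade logic.
; BeginPlay initializes PlayerAttributeSet from a stat DataTable, and possession applies a default GameplayEffect to itself.
; A debug key draws a sphere trace at the primary target.
; Disconnected example graphs sketch weapon and tome upgrades through SetByCaller effects, with partly unfinished tome stacking and a three-slot check.
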(event EventBeginPlay
  (Class|AbilitySystemComponent|InitStats (Variables|Default|GetAbilitySystemComponent) "/Script/Megabonky.PlayerAttributeSet" "/Game/Blueprints/AbilitySystem/Data/DT_Stat_Player_Default.DT_Stat_Player_Default"))

(event EventPossessed
  (params (NewController :type Controller%20Object%20Reference))
  ;[1 1 1] Init Attributes --> ASC::InitStat 함수가 있음
  (GameplayEffects|ApplyGameplayEffectSpecToSelf (Variables|Default|GetAbilitySystemComponent) (GameplayEffects|MakeOutgoingSpec (Variables|Default|GetAbilitySystemComponent) "/Game/Blueprints/AbilitySystem/GameplayEffects/Player/GE_Player_Default.GE_Player_Default_C" 1.0 (GameplayEffects|MakeEffectContext (Variables|Default|GetAbilitySystemComponent)))))

(event Input|KeyboardEvents|DebugKey2
  (params (Key :type Key%20Structure :default "None") (ActionValue :type Input%20Action%20Value%20Structure))
  ;[0.15 0.15 0.15 0.5] Primary Target 확인용
  (:Pressed
    (bind (_outprimarytarget _returnvalue) (Class|MgbPlayerCharacter|FindPrimaryTargetbyCondition))
    (if _returnvalue
      (Collision|SphereTraceByChannel (Transformation|GetActorLocation _outprimarytarget) (Transformation|GetActorLocation _outprimarytarget) 3e+01 "TraceTypeQuery1" false (Utilities|Array|MakeArray 0) "ForDuration" true "(R=1.000000,G=0.000000,B=0.000000,A=1.000000)" "(R=0.000000,G=1.000000,B=0.000000,A=1.000000)" 3.0))))

(event Input|KeyboardEvents|DebugKey3
  (params (Key :type Key%20Structure :default "None") (ActionValue :type Input%20Action%20Value%20Structure))
  ;[0.15 0.15 0.15 0.5] 비전서 업그레이드 코드 예시
)

(fn ConstructionScript)