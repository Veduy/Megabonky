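; Test enemy Character that chases the first player pawn.
; Every Tick it pushes its capsule with a constant horizontal force toward the player and sets its yaw to face them.
; Unconnected logic holds an alternative movement-input chase and a wall climb that uses forward and downward line traces to switch between Flying, Falling and Walking.
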(event EventTick
  (params (DeltaSeconds :type Float%20%28single-precision%29))
  (Utilities|FlowControl|Sequence
    (:then_0
      (Physics|AddForce (Variables|Collision|GetCapsuleComponent) (* (Class|KismetMathLibrary|VectorNormal2D (- (Transformation|GetActorLocation (Game|Player|GetPlayerPawn 0)) (Transformation|GetActorLocation)) 0.01) 5e+03) "None" false))
    (:then_1
      ;[1 1 1] Look Player
      (Transformation|SetActorRotation (Math|Rotator|MakeRotator 0.0 0.0 (.yaw (Math|Rotator|FindLookatRotation (Transformation|GetActorLocation) (Transformation|GetActorLocation (Game|Player|GetPlayerPawn 0)))))))))

(fn ConstructionScript)