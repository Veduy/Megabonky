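; Test enemy pawn that chases player 0 and climbs over obstacles in its way.
; Each Tick it offsets itself horizontally toward the player at constant speed without sweep and turns its yaw to face them.
; A short forward line trace at foot height detects WorldStatic walls and nudges the pawn upward while blocked.
; A downward ground trace meant for forced falling is unconnected and unfinished, so nothing brings it back down.
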(event EventTick
  (params (DeltaSeconds :type Float%20%28single-precision%29))
  (bind _returnvalue (Transformation|GetActorLocation))
  (bind _returnvalue_2 (- _returnvalue (Math|Vector|MakeVector 0.0 0.0 88.0)))
  (Utilities|FlowControl|Sequence
    (:then_0
      ;[1 1 1] Add Movement to Player
      (Transformation|AddActorWorldOffset (* (* (Class|KismetMathLibrary|VectorNormal2D (- (Transformation|GetActorLocation (Game|Player|GetPlayerPawn 0)) (Transformation|GetActorLocation)) 0.01) 2e+02) (Utilities|Time|GetWorldDeltaSeconds))))
    (:then_1
      ;[1 1 1] Look Player
      (Transformation|SetActorRotation (Math|Rotator|MakeRotator 0.0 0.0 (.yaw (Math|Rotator|FindLookatRotation (Transformation|GetActorLocation) (Transformation|GetActorLocation (Game|Player|GetPlayerPawn 0)))))))
    (:then_2
      ;[1 1 1] Enemy 움직임
      ;;[1 1 1] 벽 탐지
      (bind _returnvalue_3 (Collision|LineTraceForObjects _returnvalue_2 (+ _returnvalue_2 (* (Transformation|GetActorForwardVector) 7e+01)) (Utilities|Array|MakeArray "ObjectTypeQuery1") false (Utilities|Array|MakeArray 0) "ForOneFrame"))
      (if _returnvalue_3
        ;;[1 1 1] 타겟과 벽을 사이에 두고있을때는 벽을 넘을수 있도록 .UpVector add Input
        (Transformation|AddActorWorldOffset (* (* (Transformation|GetActorUpVector) 1e+02) (Utilities|Time|GetWorldDeltaSeconds)))))))

(fn ConstructionScript)